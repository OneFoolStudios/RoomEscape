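; Interactive laptop prop whose lid swings open or shut and which brings up a command-prompt widget (BP_CMD) once opened.
; OpenCloseLaptop plays or reverses the OpenRotation timeline, which pitches the Arrow component by the opening angle plus a correction offset, also applied at construction.
; The timeline's halfway point flips LaptopClosed, and finishing in the open state creates the widget for the first player.
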(event `self.ReceiveBeginPlay`)

(event `OpenCloseLaptop`
  (if (`self.LaptopClosed`)
    (bind (_direction _rotationfactor) (`Timeline|OpenRotation` :!label _label)
      (:`Update`
        (`SceneComponent.K2_SetRelativeRotation` (`self.Arrow`) (`KismetMathLibrary.MakeRotator` 0.0 (+ (* _rotationfactor (`self.OpeningDegrees`)) (`self.CorrectionDegrees`)) 90.0) false false)
        (if (< _rotationfactor 0.5)
          (set `self.LaptopClosed` true)
          (else
            (set `self.LaptopClosed` false))))
      (:`Finished`
        (if (not (`self.LaptopClosed`))
          (bind _returnvalue (`|CreateWidget` "/Game/WordMiniGame/BP_CMD.BP_CMD_C" (`GameplayStatics.GetPlayerController` 0)))
          (`UserWidget.AddToViewport` _returnvalue 0))))
    (else
      (goto _label :!via `Reverse`))))

(fn `UserConstructionScript`
  (`SceneComponent.K2_AddRelativeRotation` (`self.Arrow`) (`KismetMathLibrary.MakeRotator` 0.0 (`self.CorrectionDegrees`)) false false))