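; Interactive chest Blueprint that swings open and closed each time OpenCloseChest is called.
; The OpenRoatation timeline plays or reverses based on ChestClosed, pitching the Arrow component by OpeningDegrees plus CorrectionDegrees.
; ChestClosed flips at the timeline's halfway factor, so a call mid-swing picks direction from the current position.
; The construction script applies the correction pitch, and BeginPlay prints the root component's name.
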(event `self.ReceiveBeginPlay`
  (`KismetSystemLibrary.PrintString` (`KismetSystemLibrary.GetObjectName` (`self.K2_GetRootComponent`))))

(event `OpenCloseChest`
  (if (`self.ChestClosed`)
    (bind (_direction _rotationfactor) (`Timeline|OpenRoatation` :!label _label)
      (:`Update`
        (`SceneComponent.K2_SetRelativeRotation` (`self.Arrow`) (`KismetMathLibrary.MakeRotator` 0.0 (+ (* _rotationfactor (`self.OpeningDegrees`)) (`self.CorrectionDegrees`)) -90.0) false false)
        (if (< _rotationfactor 0.5)
          (set `self.ChestClosed` true)
          (else
            (set `self.ChestClosed` false)))))
    (else
      (goto _label :!via `Reverse`))))

(fn `UserConstructionScript`
  (`SceneComponent.K2_AddRelativeRotation` (`self.Arrow`) (`KismetMathLibrary.MakeRotator` 0.0 (`self.CorrectionDegrees`)) false false))