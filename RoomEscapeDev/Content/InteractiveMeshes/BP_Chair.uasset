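; BP_Chair is an interactive chair that gets pushed away in the direction the player character is facing.
; The MoveChair event restarts the Pushing timeline, which on each update offsets the chair's world location along the player's forward vector, scaled by PushFactor and the timeline's curve value.
; The movement uses no sweep, so the chair does not stop at obstacles.
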(event `MoveChair`
  (bind (_direction _pushfactor) (`Timeline|Pushing` :!via `PlayFromStart`)
    (:`Update`
      (`SceneComponent.K2_SetWorldLocation` (`self.Chair`) (+ (`SceneComponent.K2_GetComponentLocation` (`self.Chair`)) (* (`self.GetActorForwardVector` (`GameplayStatics.GetPlayerCharacter` 0)) (* (`self.PushFactor`) _pushfactor))) false false))))

(fn `UserConstructionScript`)