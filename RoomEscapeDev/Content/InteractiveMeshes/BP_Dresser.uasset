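; BP_Dresser is a dresser with sliding drawers, currently running a BeginPlay test that opens the top-left drawer, then requests it closed after a delay.
; OpenDrawer and CloseDrawer play separate timelines that add scaled local Y offsets every update, so movement accumulates per tick.
; Both events gate on CheckIfDrawerIsOpen, whose graph shows only an unused comparison of drawer location against zero.
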(event `self.ReceiveBeginPlay`
  (bind _topleftdrawer (`self.TopLeftDrawer`))
  (`KismetSystemLibrary.Delay` 2.0)
  (`self.OpenDrawer` _topleftdrawer)
  (`KismetSystemLibrary.Delay` 5.0)
  (`self.CloseDrawer` _topleftdrawer))

(event `OpenDrawer`
  (params (Drawer :type "StaticMeshComponent Object Reference"))
  (if (not (`self.CheckIfDrawerIsOpen` Drawer))
    (bind (_direction _opendrawer) (`Timeline|OpeningDrawer` :!via `PlayFromStart`)
      (:`Update`
        (`SceneComponent.K2_AddLocalOffset` Drawer (`KismetMathLibrary.MakeVector` 0.0 (* _opendrawer (`self.DrawingOpeningFactor`))) false false)))))

(event `CloseDrawer`
  (params (Drawer :type "StaticMeshComponent Object Reference"))
  (if (`self.CheckIfDrawerIsOpen` Drawer)
    (bind (_direction _closedrawer) (`Timeline|ClosingDrawer` :!via `PlayFromStart`)
      (:`Update`
        (`SceneComponent.K2_AddLocalOffset` Drawer (`KismetMathLibrary.MakeVector` 0.0 (* _closedrawer (`self.DrawingOpeningFactor`))) false false)))))

(fn `UserConstructionScript`)