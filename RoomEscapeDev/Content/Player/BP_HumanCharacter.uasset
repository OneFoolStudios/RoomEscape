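; BP_HumanCharacter is the player character, handling movement, looking, jump, crouch and object interaction, and adding the BP_PlayerUI widget on BeginPlay.
; Movement and look inputs forward to functions defined outside these graphs.
; Interaction takes the hit object from Interact and switches on its root name to call chest, dresser, globe or laptop handlers.
; Handlers cast to each prop Blueprint, with the dresser also switching on mesh name to pick the drawer.
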(event `self.ReceiveBeginPlay`
  (bind _returnvalue (`|CreateWidget` "/Game/Player/BP_PlayerUI.BP_PlayerUI_C" (`GameplayStatics.GetPlayerController` 0)))
  (`UserWidget.AddToViewport` _returnvalue 0))

(event `InputAxis|MoveForward`
  (params (AxisValue :type "Float (single-precision)"))
  ;[1 1 1] Movement Input Setup
  (`self.MoveForward` AxisValue))

(event `InputAction|Interaction`
  (params (Key :type "Key Structure" :default "AnyKey"))
  ;[1 1 1] Interactions
  (:`Pressed`
    (bind (_rootname _returnvalue) (`Interact.GetHitObject` (`self.Interact`)))
    (switch `name` (`KismetStringLibrary.Conv_StringToName` _rootname)
      (:`ChestBox`
        (bind _returnvalue_2 (`ActorComponent.GetOwner` _returnvalue))
        (`self.InteractChest` _returnvalue_2))
      (:`DresserChassis`
        (`self.InteractDresser` _returnvalue _returnvalue_2))
      (:`GlobeHolder`
        (`self.InteractGlobe` _returnvalue_2))
      (:`LaptopChassis`
        (`self.InteractLaptop` _returnvalue_2)))))

(event `InputAxis|MoveRight`
  (params (AxisValue :type "Float (single-precision)"))
  ;[1 1 1] Movement Input Setup
  (`self.MoveLeft` AxisValue))

(event `InputAction|Jump`
  (params (Key :type "Key Structure" :default "AnyKey"))
  ;[1 1 1] Movement Input Setup
  (:`Pressed`
    (`self.Jump`)))

(event `InputAction|Crouch`
  (params (Key :type "Key Structure" :default "AnyKey"))
  ;[1 1 1] Movement Input Setup
  (:`Pressed`
    (`self.Crouch`))
  (:`Released`
    (`self.UnCrouch`)))

(event `InputAxis|LookUp`
  (params (AxisValue :type "Float (single-precision)"))
  ;[1 1 1] Looking Input Setup
  (`self.LookUp` AxisValue))

(event `InputAxis|LookRight`
  (params (AxisValue :type "Float (single-precision)"))
  ;[1 1 1] Looking Input Setup
  (`self.LookLeft` AxisValue))

(fn `InteractChest`
  (params (ChestActor :type "Object Object Reference"))
  (`/Game/InteractiveMeshes/BP_Chest.OpenCloseChest` (cast `/Game/InteractiveMeshes/BP_Chest` ChestActor :!pure true)))

(fn `InteractDresser`
  (params (DrawerMesh :type "Object Object Reference") (DresserActor :type "Object Object Reference"))
  (bind _asbp_dresser (cast `/Game/InteractiveMeshes/BP_Dresser` DresserActor :!pure true))
  (switch `string` (`KismetSystemLibrary.GetObjectName` DrawerMesh)
    (:`TopLeftDrawer`
      (`/Game/InteractiveMeshes/BP_Dresser.OpenCloseTopLeftDrawer` _asbp_dresser))
    (:`TopMiddleDrawer`
      (`/Game/InteractiveMeshes/BP_Dresser.OpenCloseTopMiddleDrawer` _asbp_dresser))
    (:`TopRightDrawer`
      (`/Game/InteractiveMeshes/BP_Dresser.OpenCloseTopRightDrawer` _asbp_dresser))
    (:`BottomDrawer`
      (`/Game/InteractiveMeshes/BP_Dresser.OpenCloseBottomDrawer` _asbp_dresser))
    (:`MiddleDrawer`
      (`/Game/InteractiveMeshes/BP_Dresser.OpenCloseMiddleDrawer` _asbp_dresser))))

(fn `InteractGlobe`
  (params (Object :type "Object Object Reference"))
  (`/Game/InteractiveMeshes/BP_Globe.RotateGlobe` (cast `/Game/InteractiveMeshes/BP_Globe` Object :!pure true)))

(fn `InteractLaptop`
  (params (Object :type "Object Object Reference"))
  (`/Game/InteractiveMeshes/BP_Laptop.OpenCloseLaptop` (cast `/Game/InteractiveMeshes/BP_Laptop` Object :!pure true)))

(fn `UserConstructionScript`)